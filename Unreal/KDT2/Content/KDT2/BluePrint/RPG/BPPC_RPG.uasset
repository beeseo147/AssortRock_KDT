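; BPPC_RPG is the player controller for the RPG, handling camera zoom and attack input.
; On BeginPlay it adds the IMC_RPG Enhanced Input mapping context and snaps the pawn's spring arm to the target length.
; The zoom wheel adjusts a clamped target length, which Tick smoothly interpolates the spring arm toward.
; The attack action casts the controlled pawn to BPC_RPG and calls its Attack.
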(event `self.ReceiveBeginPlay`
  (`EnhancedInputSubsystemInterface.AddMappingContext` (subsystem `EnhancedInputLocalPlayerSubsystem`) "/Game/KDT2/Blueprint/RPG/Input/IMC_RPG.IMC_RPG" 0 (struct))
  (set `SpringArmComponent.TargetArmLength` (`self.TargetArmLength`) (`self.GetComponentByClass` (`self.K2_GetPawn`) "/Script/Engine.SpringArmComponent")))

(event `self.ReceiveTick`
  (params (DeltaSeconds :type "Float (single-precision)"))
  (bind _returnvalue (`self.GetComponentByClass` (`self.K2_GetPawn`) "/Script/Engine.SpringArmComponent"))
  (set `SpringArmComponent.TargetArmLength` (`KismetMathLibrary.Lerp` (`SpringArmComponent.TargetArmLength` _returnvalue) (`self.TargetArmLength`) (* DeltaSeconds 3.0)) _returnvalue))

(event `EnhancedInput|/Game/KDT2/Blueprint/RPG/Input/IA_ZoomWheel`
  (params (ActionValue :type "Float (double-precision)") (ElapsedSeconds :type "Float (double-precision)") (TriggeredSeconds :type "Float (double-precision)") (InputAction :type "InputAction Object Reference" :default "/Game/KDT2/Blueprint/RPG/Input/IA_ZoomWheel.IA_ZoomWheel"))
  (:`Triggered`
    (set `self.TargetArmLength` (`KismetMathLibrary.FClamp` (+ (`self.TargetArmLength`) (* ActionValue -1.0 50.0)) 150.0 1200.0))))

(event `EnhancedInput|/Game/KDT2/Blueprint/RPG/Input/IA_Attack`
  (params (ActionValue :type Boolean) (ElapsedSeconds :type "Float (double-precision)") (TriggeredSeconds :type "Float (double-precision)") (InputAction :type "InputAction Object Reference" :default "/Game/KDT2/Blueprint/RPG/Input/IA_Attack.IA_Attack"))
  (:`Started`
    (bind _asbpc_rpg (cast `/Game/KDT2/Blueprint/RPG/BPC_RPG` (`self.K2_GetPawn`)))
    (`/Game/KDT2/Blueprint/RPG/BPC_RPG.Attack` _asbpc_rpg)))

(fn `UserConstructionScript`)