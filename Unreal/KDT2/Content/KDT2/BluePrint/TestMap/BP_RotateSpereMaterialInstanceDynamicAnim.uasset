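; Test actor with a spinning mesh orbited by a self-rotating satellite mesh, plus an animated dynamic sprite-texture material.
; The construction script creates the material instance and applies color, texture and UV, though the texture parameter name is None.
; BeginPlay starts a looping timer that cycles red, blue and green, and a timeline animating the UV vector's third channel.
; Tick spins both meshes and rotates a scene pivot for the orbit.
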(event `ChangeColor`
  (bind _mid_staticmesh (`self.MID_StaticMesh`))
  (`|MultiGate` false true
    (:`Out 0`
      (`MaterialInstanceDynamic.SetVectorParameterValue` _mid_staticmesh "Color" (struct :`R` 1.0 :`A` 1.0)))
    (:`Out 1`
      (`MaterialInstanceDynamic.SetVectorParameterValue` _mid_staticmesh "Color" (struct :`G` 0.026303 :`B` 1.0 :`A` 1.0)))
    (:`Out 2`
      (`MaterialInstanceDynamic.SetVectorParameterValue` _mid_staticmesh "Color" (struct :`R` 0.141643 :`G` 1.0 :`A` 1.0)))))

(event `self.ReceiveBeginPlay`
  (bind (_uv_r _uv_g _uv_b _uv_a) (break `LinearColor` (`self.UV`)))
  (`KismetSystemLibrary.K2_SetTimerDelegate` (delegate `ChangeColor`) 1.0 true)
  (bind (_direction _value) (`Timeline|UVTimeLine`)
    (:`Update`
      (bind _output_get (set `self.UV` (make `LinearColor` _uv_r _uv_g _value _uv_a)))
      (`MaterialInstanceDynamic.SetVectorParameterValue` (`self.MID_StaticMesh`) "UV" _output_get))))

(event `self.ReceiveTick`
  (params (DeltaSeconds :type "Float (single-precision)"))
  (`|ExecutionSequence`
    (:`then_0`
      ;[1 1 1] staticMesh를 회전시킨다
      (`SceneComponent.K2_AddRelativeRotation` (`self.StaticMesh`) (`KismetMathLibrary.MakeRotator` 0.0 0.0 (* (`GameplayStatics.GetWorldDeltaSeconds`) 10.0)) false false))
    (:`then_1`
      ;[1 1 1] Scene1을  회전시켜 위성(StaticMesh1)을 공전시킨다
      (`SceneComponent.K2_AddLocalRotation` (`self.Scene1`) (`KismetMathLibrary.MakeRotator` 0.0 0.0 (* (`GameplayStatics.GetWorldDeltaSeconds`) (`self.SceneRotationSpeed1`))) false false)
      ;[1 1 1] Scene1을  회전시켜 위성(StaticMesh1)을 자전시킨다
      (`SceneComponent.K2_AddRelativeRotation` (`self.StaticMesh1`) (`KismetMathLibrary.MakeRotator` 0.0 (* (`self.StaticRotationSpeed1`) (`GameplayStatics.GetWorldDeltaSeconds`))) false false))))

(fn `NewFunction`
  (params (InDouble :type "Float (double-precision)") (A :type "Float (double-precision)"))
  ;[1 1 1] staticMesh를 ㅣ전시킨다
  (`KismetSystemLibrary.PrintString` (`KismetStringLibrary.Conv_DoubleToString` InDouble))
  (`SceneComponent.K2_AddRelativeRotation` (`self.StaticMesh`) (`KismetMathLibrary.MakeRotator` 0.0 0.0 (* A 10.0)) false false))

(fn `UserConstructionScript`
  (bind _returnvalue (`PrimitiveComponent.CreateDynamicMaterialInstance` (`self.StaticMesh`) 0 "/Game/KDT2/BluePrint/TestMap/MT_SpriteTexure.MT_SpriteTexure" "None"))
  (`/Engine/EditorBlueprintResources/StandardMacros.IsValid` _returnvalue
    (:`Is Valid`
      (bind _output_get (set `self.MID_StaticMesh` _returnvalue))
      (`MaterialInstanceDynamic.SetVectorParameterValue` _output_get "Color" (`self.Color`))
      (`MaterialInstanceDynamic.SetTextureParameterValue` _output_get "None" (`self.Texture`))
      (`MaterialInstanceDynamic.SetVectorParameterValue` (`self.MID_StaticMesh`) "UV" (`self.UV`)))))