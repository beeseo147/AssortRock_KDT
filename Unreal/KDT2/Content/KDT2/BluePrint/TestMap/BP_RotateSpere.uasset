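; BP_RotateSpere is a test actor that animates a spinning body with an orbiting satellite.
; Each Tick yaws StaticMesh at a fixed rate, yaws the Scene1 pivot to orbit StaticMesh1, and pitches that satellite around itself.
; Rotations scale by world delta time, with orbit and satellite spin speeds held in variables.
; Construction and BeginPlay print debug strings, and NewFunction, a print-and-rotate helper, is not called here.
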(event `self.ReceiveBeginPlay`
  (`KismetSystemLibrary.PrintString` "BeginPlay" true true (struct :`R` 1.0 :`B` 0.801369 :`A` 1.0)))

(event `self.ReceiveTick`
  (params (DeltaSeconds :type "Float (single-precision)"))
  (`|ExecutionSequence`
    (:`then_0`
      ;[1 1 1] staticMesh를 회전시킨다
      (`SceneComponent.K2_AddRelativeRotation` (`self.StaticMesh`) (`KismetMathLibrary.MakeRotator` 0.0 0.0 (* (`GameplayStatics.GetWorldDeltaSeconds`) 10.0)) false false))
    (:`then_1`
      ;[1 1 1] Scene1을  회전시켜 위성(StaticMesh1)을 공전시킨다
      (`SceneComponent.K2_AddLocalRotation` (`self.Scene1`) (`KismetMathLibrary.MakeRotator` 0.0 0.0 (* (`GameplayStatics.GetWorldDeltaSeconds`) (`self.SceneRotationSpeed1`))) false false)
      ;[1 1 1] Scene1을  회전시켜 위성(StaticMesh1)을 자전시킨다
      (`SceneComponent.K2_AddRelativeRotation` (`self.StaticMesh1`) (`KismetMathLibrary.MakeRotator` 0.0 (* (`self.StaticRotationSpeed1`) (`GameplayStatics.GetWorldDeltaSeconds`))) false false))))

(fn `NewFunction`
  (params (InDouble :type "Float (double-precision)") (A :type "Float (double-precision)"))
  ;[1 1 1] staticMesh를 ㅣ전시킨다
  (`KismetSystemLibrary.PrintString` (`KismetStringLibrary.Conv_DoubleToString` InDouble))
  (`SceneComponent.K2_AddRelativeRotation` (`self.StaticMesh`) (`KismetMathLibrary.MakeRotator` 0.0 0.0 (* A 10.0)) false false))

(fn `UserConstructionScript`
  (`KismetSystemLibrary.PrintString` "Construct"))