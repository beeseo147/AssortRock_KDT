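; BP_Sun is a sun actor for a solar system whose mesh material has a scriptable Power parameter.
; The construction script creates a dynamic material instance from the static mesh's first material and stores it as MIDSun.
; On BeginPlay, the Power timeline plays and writes its scaled value to that parameter on each update.
; The timeline's play rate is set to zero beforehand, so its playback does not advance.
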(event `self.ReceiveBeginPlay`
  (`TimelineComponent.SetPlayRate` (`self.Power`) 0.0)
  (bind (_direction _value) (`Timeline|Power`)
    (:`Update`
      (`MaterialInstanceDynamic.SetScalarParameterValue` (`self.MID_Sun`) "Power" (* _value 50.0)))))

(fn `UserConstructionScript`
  (bind _staticmesh (`self.StaticMesh`))
  (bind _returnvalue (`PrimitiveComponent.CreateDynamicMaterialInstance` _staticmesh 0 (`PrimitiveComponent.GetMaterial` _staticmesh 0) "None"))
  (set `self.MID_Sun` _returnvalue))